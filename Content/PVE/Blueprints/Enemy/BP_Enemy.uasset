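; BP_Enemy is a PVE enemy Blueprint that relays hit notifications and handles its own death.
; HitNotifiy fires the OnHitOpponent dispatcher.
; CheckDead reads a base float attribute from the Ability System Component; at zero or below, it sets IsDead once, detaches the controller, then enables mesh gravity after a short delay.
; BeginPlay and overlap events are empty, and an attribute debug print is unconnected.
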(event Custom|CheckDead
  (if (not (Variables|Default|GetIsDead))
    (if (<= (.ReturnValue (Class|AbilitySystemBlueprintLibrary|GetFloatAttributeBasefromAbilitySystemComponent (Variables|Default|GetAbilitySystemComponent) "(AttributeName=\"Health\",Attribute=/Script/PVECPP.PlayerAttributeSet:Health,AttributeOwner=\"/Script/CoreUObject.Class'/Script/PVECPP.PlayerAttributeSet'\")")) 0.0)
      (Variables|Default|SetIsDead true)
      (Class|Pawn|DetachfromControllerPendingDestroy)
      (Utilities|FlowControl|Delay 0.5)
      (Physics|SetEnableGravity (Variables|Character|GetMesh) true))))

(event Custom|HitNotifiy
  (Default|CallOnHitOpponent))

(event EventBeginPlay)

(event Collision|EventActorBeginOverlap
  (params (OtherActor :type Actor%20Object%20Reference)))

(fn ConstructionScript)