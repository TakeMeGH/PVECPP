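; PVE game mode that runs a timed round where the player earns a point for each enemy killed.
; Reset respawns the player at a PlayerStart, clears enemies, gathers "Spawner"-tagged actors, rebinds health events and rebuilds the HUD.
; Tick counts down the round and periodically spawns enemies at random spawners, binding their death events to scoring.
; When time runs out, it stops the player and shows the game-over menu with the score.
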(event Custom|OnHealthChange
  (bind _bpplayer (Variables|Default|GetBPPlayer))
  (bind _abilitysystemcomponent (Variables|/Script/PVECPP.PVECPPCharacter|GetAbilitySystemComponent _bpplayer))
  (Utilities|IsValid _bpplayer
    (:Is%20Valid
      (Default|SetHealth (Variables|Default|GetHUD) (.ReturnValue (Class|AbilitySystemComponent|GetGameplayAttributeValue _abilitysystemcomponent "(AttributeName=\"Health\",Attribute=/Script/PVECPP.PlayerAttributeSet:Health,AttributeOwner=\"/Script/CoreUObject.Class'/Script/PVECPP.PlayerAttributeSet'\")")) (.ReturnValue (Class|AbilitySystemComponent|GetGameplayAttributeValue _abilitysystemcomponent "(AttributeName=\"MaxHealth\",Attribute=/Script/PVECPP.PlayerAttributeSet:MaxHealth,AttributeOwner=\"/Script/CoreUObject.Class'/Script/PVECPP.PlayerAttributeSet'\")"))))))

(event EventBeginPlay
  (CallFunction|Reset))

(event EventTick
  (params (DeltaSeconds :type Float%20%28single-precision%29))
  (if (or (<= (Variables|Default|GetCurrentTimer) 0.0) (Variables|Default|GetIsGameStop))
    (CallFunction|OnGameStop)
    (else
      (Variables|Default|SetCurrentTimer (- (Variables|Default|GetCurrentTimer) DeltaSeconds))
      (CallFunction|CheckSpawn))))

(fn ConstructionScript)

(fn Reset
  (bind _gameovermenu (Variables|Default|GetGameOverMenu))
  (Utilities|FlowControl|Sequence
    (:then_0
      ;[1 1 1] Variable Set
      (Variables|Default|SetIsEnded false)
      (Variables|Default|SetCurrentTimer (Variables|Default|GetMaxTimer))
      (Variables|Default|SetCurrentSpawnTime 5.0)
      (Variables|Default|SetPoint 0)
      (Variables|Default|SetIsGameStop false)
      (Utilities|IsValid (Variables|Default|GetHUD)
        (:Is%20Valid
          (Widget|RemovefromParent (Variables|Default|GetHUD)))))
    (:then_1
      ;[1 1 1] Player Set
      (bind _asbp_player (Utilities|Casting|CastToBP_Player (Game|GetPlayerCharacter 0)))
      (Variables|Default|SetBPPlayer _asbp_player))
    (:then_2
      ;[1 1 1] Respawn player
      (bind _asbp_player_2 (Utilities|Casting|CastToBP_Player (Game|GetPlayerCharacter 0)))
      (Actor|DestroyActor _asbp_player_2)
      (bind _returnvalue (Game|SpawnActorfromClass "/Game/PVE/Blueprints/Player/BP_Player.BP_Player_C" (Math|Conversions|ToTransform(Vector) (Transformation|GetActorLocation (Class|GameModeBase|FindPlayerStart))) "Undefined" "MultiplyWithRoot" 0 0))
      (Pawn|Possess (Game|GetPlayerController 0) _returnvalue)
      (Variables|Default|SetBPPlayer _returnvalue))
    (:then_3
      ;[1 1 1] Rebind Event
      (EventDispatchers|UnbindallEventsfromHealthChangeEvent)
      (EventDispatchers|BindEventtoHealthChangeEvent (EventDispatchers|CreateEvent :!event Custom|OnHealthChange)))
    (:then_4
      ;[1 1 1] Get Spawner
      (bind _outactors (Actor|GetAllActorsOfClasswithTag "/Script/Engine.Actor" "Spawner"))
      (Variables|Default|SetSpawners _outactors))
    (:then_5
      ;[1 1 1] Destroy all enemy
      (bind _outactors_2 (Actor|GetAllActorsOfClass "/Game/PVE/Blueprints/Enemy/BP_Enemy.BP_Enemy_C"))
      (for _array_element _outactors_2
        (Actor|DestroyActor _array_element)))
    (:then_6
      ;[1 1 1] Reset UI
      (Utilities|IsValid _gameovermenu
        (:Is%20Valid
          (Widget|RemovefromParent _gameovermenu))
        (:Is%20Not%20Valid
          _))
      (bind _returnvalue_2 (UserInterface|CreateWidget "/Game/PVE/Blueprints/UI/WBP_HUD.WBP_HUD_C"))
      (bind _output_get (Variables|Default|SetHUD _returnvalue_2))
      (UserInterface|Viewport|AddtoViewport _output_get 0)
      (CallFunction|OnHealthChange)
      (Default|SetPoint (Variables|Default|GetHUD) (Variables|Default|GetPoint))
      (Variables|/Script/Engine.PlayerController|SetbShowMouseCursor (Game|GetPlayerController 0) false))))

(fn CheckSpawn
  (bind _output_get (Variables|Default|SetCurrentSpawnTime (- (Variables|Default|GetCurrentSpawnTime) (Utilities|Time|GetWorldDeltaSeconds))))
  (if (<= _output_get 0.0)
    (Variables|Default|SetCurrentSpawnTime (Variables|Default|GetMaxSpawnTime))
    (bind _returnvalue (Game|SpawnActorfromClass "/Game/PVE/Blueprints/Enemy/BP_Enemy.BP_Enemy_C" (Math|Transform|MakeTransform (Transformation|GetActorLocation (.OutItem (Utilities|Array|Random (Variables|Default|GetSpawners)))) "0, 0, 0" "1.000000,1.000000,1.000000") "Undefined" "MultiplyWithRoot" 0 0))
    (EventDispatchers|BindEventtoOnEnemyDead _returnvalue (EventDispatchers|CreateEvent :!event OnEnemyKilled))))

(fn OnEnemyKilled
  (bind _result (Math|Integer|IncrementInt (Variables|Default|GetPoint))
    (:%20%20
      (Default|SetPoint (Variables|Default|GetHUD) _result))))

(fn OnGameStop
  (if (not (Variables|Default|GetIsGameStop))
    (Default|StopPlayer (Variables|Default|GetBPPlayer))
    (Variables|Default|SetIsGameStop true)
    (Widget|RemovefromParent (Variables|Default|GetHUD))
    (bind _returnvalue (UserInterface|CreateWidget "/Game/PVE/Blueprints/UI/WBP_GameOverMenu.WBP_GameOverMenu_C"))
    (bind _output_get (Variables|Default|SetGameOverMenu _returnvalue))
    (Default|SetPoint _output_get (Variables|Default|GetPoint))
    (Variables|/Script/Engine.PlayerController|SetbShowMouseCursor (Game|GetPlayerController 0) true)
    (UserInterface|Viewport|AddtoViewport _output_get 0)))