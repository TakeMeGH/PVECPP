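; Gameplay ability that maintains the player's lock-on to an enemy target.
; On activation it disables orient-to-movement and searches the player's surroundings for the current LockTarget.
; If the target is found, it calls LookTarget and ends after a tiny delay, so each activation is a single look update.
; Otherwise it clears IsLock, restores orient-to-movement and ends immediately.
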(event Ability|EventActivateAbility
  (Ability|CommitAbility)
  (bind _asbp_player (Utilities|Casting|CastToBP_Player (.OwnerActor (Utilities|Struct|BreakGameplayAbilityActorInfo (Ability|GetActorInfo)))))
  (bind _output_get (Variables|Default|SetBPPlayer _asbp_player))
  (Variables|/Script/Engine.CharacterMovementComponent|SetbOrientRotationToMovement (Variables|/Script/Engine.Character|GetCharacterMovement _output_get) false)
  (bind _enemies (Default|CheckArround (Variables|Default|GetBPPlayer) 1e+03))
  (Variables|Default|SetIsLockStillExist false)
  (for _array_element _enemies
    (bind _asbp_enemy (Utilities|Casting|CastToBP_Enemy _array_element))
    (if (== _asbp_enemy (Variables|/Game/PVE/Blueprints/Player/BP_Player.BP_Player_C|GetLockTarget (Variables|Default|GetBPPlayer)))
      (Variables|Default|SetIsLockStillExist true)))
  (if (Variables|Default|GetIsLockStillExist)
    (Default|LookTarget (Variables|Default|GetBPPlayer))
    (Ability|Tasks|WaitDelay 0.001
      (:OnFinish
        (Ability|EndAbility)))
    (else
      (Variables|/Game/PVE/Blueprints/Player/BP_Player.BP_Player_C|SetIsLock (Variables|Default|GetBPPlayer) false)
      (Variables|/Script/Engine.CharacterMovementComponent|SetbOrientRotationToMovement (Variables|/Script/Engine.Character|GetCharacterMovement (Variables|Default|GetBPPlayer)) true)
      (Ability|EndAbility))))