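; GA_Knockback is a gameplay ability that pushes a BP_Enemy away from whatever pawn knocked it back.
; On activation it commits and waits once for a Character.Events.Knockback gameplay event, taking the source pawn from the payload's OptionalObject.
; It applies a constant root motion force along the normalized source-to-enemy direction at KnockbackStrength, keeps the final velocity, then ends when the force finishes.
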(event Ability|EventActivateAbility
  (Ability|CommitAbility)
  (bind _payload (Ability|Tasks|WaitGameplayEvent "(TagName=\"Character.Events.Knockback\")" 0 true)
    (:EventReceived
      (bind _aspawn (Utilities|Casting|CastToPawn (.OptionalObject (Utilities|Struct|BreakGameplayEventData _payload))))
      (Variables|Default|SetSurceKnockback (Transformation|GetActorLocation _aspawn))
      (bind _asbp_enemy (Utilities|Casting|CastToBP_Enemy (.OwnerActor (Utilities|Struct|BreakGameplayAbilityActorInfo (Ability|GetActorInfo)))))
      (Variables|Default|SetTargetKnockback (Transformation|GetActorLocation _asbp_enemy))
      (bind _direction (CallFunction|CalculateDirection))
      (Ability|Tasks|ApplyRootMotionConstantForce "None" _direction (Variables|Default|GetKnockbackStrength) 0.0 false 0 "MaintainLastRootMotionVelocity"
        (:OnFinish
          (Ability|EndAbility))))))

(fn CalculateDirection
  (return (Math|Vector|Normalize (- (Variables|Default|GetTargetKnockback) (Variables|Default|GetSurceKnockback)))))