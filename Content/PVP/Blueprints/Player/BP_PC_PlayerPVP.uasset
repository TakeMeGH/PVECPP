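; Player controller for the PVP mode that requests the player's spawn, forwards input and creates the HUD.
; On local begin play it adds the Enhanced Input context, then calls SR_SpawnPlayer to spawn through BP_GM_PVP.
; SaveCharacter then caches the pawn and PlayerState, and seeds the HUD with Ability System health attributes and PlayerState points.
; Move and attack input pass to the cached pawn on local controllers only.
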(event Custom|SR_SpawnPlayer
  ;[1 1 1] Initialize Character
  (bind _asbp_gm_pvp (Utilities|Casting|CastToBP_GM_PVP (Game|GetGameMode)))
  (bind _bpplayer (Default|SpawnPlayer _asbp_gm_pvp self))
  (Default|BeginPlay _bpplayer)
  (CallFunction|SaveCharacter))

(event Custom|PC_BeginPlay
  ;[1 1 1] Begin Play -> Get Call On Connect Game Mode
  (if (Pawn|IsLocalPlayerController)
    (Input|AddMappingContext (PlayerController|LocalPlayerSubsystems|GetEnhancedInputLocalPlayerSubsystem self) "/Game/PVP/Inputs/IMC_PlayerPVP.IMC_PlayerPVP" 0 "(bIgnoreAllPressedKeysUntilRelease=True,bForceImmediately=False,bNotifyUserSettings=False)")
    (CallFunction|SRSpawnPlayer)))

(event Custom|SaveCharacter
  ;[1 1 1] Initialize Character
  (bind _asbp_player_pvp (Utilities|Casting|CastToBP_PlayerPVP (Pawn|GetControlledPawn)))
  (Variables|Default|SetOwnedPlayer _asbp_player_pvp)
  (bind _asbp_ps_player_pvp (Utilities|Casting|CastToBP_PS_PlayerPVP (Variables|GetPlayerState)))
  (Variables|Default|SetOwnedPS _asbp_ps_player_pvp)
  (CallFunction|InitializeUI))

(event Input|EnhancedActionEvents|EnhancedInputActionIA_Move
  (params (ActionValue :type Vector%202D%20Structure) (ElapsedSeconds :type Float%20%28double-precision%29) (TriggeredSeconds :type Float%20%28double-precision%29) (InputAction :type Input%20Action%20Object%20Reference :default "/Game/ThirdPerson/Input/Actions/IA_Move.IA_Move"))
  (bind _ownedplayer (Variables|Default|GetOwnedPlayer))
  ;[1 1 1] Input Move
  (:Triggered
    (if (Pawn|IsLocalPlayerController) :!label _label
      (Utilities|IsValid _ownedplayer
        (:Is%20Valid
          (Default|OnMove _ownedplayer ActionValue)))))
  (:Completed
    (goto _label)))

(event Input|EnhancedActionEvents|EnhancedInputActionIA_Attack
  (params (ActionValue :type Boolean) (ElapsedSeconds :type Float%20%28double-precision%29) (TriggeredSeconds :type Float%20%28double-precision%29) (InputAction :type Input%20Action%20Object%20Reference :default "/Game/PVE/Input/Actions/IA_Attack.IA_Attack"))
  (bind _ownedplayer (Variables|Default|GetOwnedPlayer))
  ;[1 1 1] Input Attack
  (:Started
    (if (Pawn|IsLocalPlayerController)
      (Utilities|IsValid _ownedplayer
        (:Is%20Valid
          (Default|OnAttack _ownedplayer))))))

(fn ConstructionScript)

(fn InitializeUI
  (bind _ownedplayer (Variables|Default|GetOwnedPlayer))
  (bind _abilitysystemcomponent (Variables|/Script/PVECPP.PVECPPCharacter|GetAbilitySystemComponent _ownedplayer))
  (bind _returnvalue (UserInterface|CreateWidget "/Game/PVE/Blueprints/UI/WBP_HUD.WBP_HUD_C"))
  (bind _output_get (Variables|Default|SetHUD _returnvalue))
  (UserInterface|Viewport|AddtoViewport _output_get 0)
  (Default|ResetUI _output_get (.ReturnValue (Ability|Attribute|GetFloatAttributefromAbilitySystemComponent _abilitysystemcomponent "(AttributeName=\"Health\",Attribute=/Script/PVECPP.PlayerAttributeSet:Health,AttributeOwner=\"/Script/CoreUObject.Class'/Script/PVECPP.PlayerAttributeSet'\")")) (.ReturnValue (Ability|Attribute|GetFloatAttributefromAbilitySystemComponent _abilitysystemcomponent "(AttributeName=\"MaxHealth\",Attribute=/Script/PVECPP.PlayerAttributeSet:MaxHealth,AttributeOwner=\"/Script/CoreUObject.Class'/Script/PVECPP.PlayerAttributeSet'\")")) (Variables|/Game/PVP/Blueprints/Player/BP_PS_PlayerPVP.BP_PS_PlayerPVP_C|GetPoint (Variables|Default|GetOwnedPS))))