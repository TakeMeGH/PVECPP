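; PvP gameplay ability that locks the player onto an enemy found nearby.
; On activation it gets nearby actors from BP_Player's CheckArround, casts each to BP_Enemy and compares its distance to a large initial threshold.
; The threshold is never updated, so NearestEnemy becomes the last enemy passing the check, not necessarily the closest.
; It then writes LockTarget and IsLock on the player and ends; an empty search just ends.
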(event Ability|EventActivateAbility
  (Ability|CommitAbility)
  (bind _asbp_player (Utilities|Casting|CastToBP_Player (.OwnerActor (Utilities|Struct|BreakGameplayAbilityActorInfo (Ability|GetActorInfo)))))
  (Variables|Default|SetBPPlayer _asbp_player)
  (Variables|Default|SetDistance 999999.0)
  (bind _enemies (Default|CheckArround (Variables|Default|GetBPPlayer) 5e+02))
  (if (>= (Utilities|Array|Length _enemies) 1)
    (for _array_element _enemies
      (bind _asbp_enemy (Utilities|Casting|CastToBP_Enemy _array_element))
      (if (<= (Math|Vector|Distance(Vector) (Transformation|GetActorLocation _asbp_enemy) (Transformation|GetActorLocation (Variables|Default|GetBPPlayer))) (Variables|Default|GetDistance))
        (Variables|Default|SetNearestEnemy _asbp_enemy)))
    (Variables|/Game/PVE/Blueprints/Player/BP_Player.BP_Player_C|SetLockTarget (Variables|Default|GetBPPlayer) (Variables|Default|GetNearestEnemy))
    (Variables|/Game/PVE/Blueprints/Player/BP_Player.BP_Player_C|SetIsLock (Variables|Default|GetBPPlayer) true)
    (Ability|EndAbility)
    (else
      (Ability|EndAbility))))