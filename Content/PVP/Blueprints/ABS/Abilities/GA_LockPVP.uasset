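; GA_LockPVP is a gameplay ability that maintains the player's lock-on to an enemy in PVP.
; On activation it disables orient-to-movement and has CheckEnemy search nearby actors for the current LockTarget.
; If found, it calls LookTarget and ends after a tiny delay; otherwise it normally clears IsLock and restores movement rotation.
; CheckEnemy's away timer only accumulates while the target is found and is reset in that same call.
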(event Ability|EventActivateAbility
  (Ability|CommitAbility)
  (bind _asbp_player (Utilities|Casting|CastToBP_Player (.OwnerActor (Utilities|Struct|BreakGameplayAbilityActorInfo (Ability|GetActorInfo)))))
  (bind _output_get (Variables|Default|SetBPPlayer _asbp_player))
  (Variables|/Script/Engine.CharacterMovementComponent|SetbOrientRotationToMovement (Variables|/Script/Engine.Character|GetCharacterMovement _output_get) false)
  (bind _islockstillexist (Utilities|CheckEnemy)
    (:Completed
      (if _islockstillexist
        (Default|LookTarget (Variables|Default|GetBPPlayer))
        (Ability|Tasks|WaitDelay 0.001
          (:OnFinish
            (Ability|EndAbility)))
        (else
          (Variables|/Game/PVE/Blueprints/Player/BP_Player.BP_Player_C|SetIsLock (Variables|Default|GetBPPlayer) false)
          (Variables|/Script/Engine.CharacterMovementComponent|SetbOrientRotationToMovement (Variables|/Script/Engine.Character|GetCharacterMovement (Variables|Default|GetBPPlayer)) true)
          (Ability|EndAbility))))))